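; BP_Spawner is a foraging spawner that creates pickup models at random spots inside its box volume.
; The SpawnPickUp input triggers SpawnActor on the first spawner found, spawning a BP_Model at a random X/Y and assigning it a random data asset and matching mesh.
; A testing input destroys all BP_PickUpObject actors.
; The RandomizePosition helper is not called in this graph.
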(event Custom|SpawnActor
  (bind _spawnervolume (Variables|Default|GetSpawnerVolume))
  ;[0 0 0] Random Spawn Position
  (bind _output_get (Variables|Default|SetRandomPoint (Math|Random|RandomPointinBoundingBox (Transformation|GetWorldLocation _spawnervolume) (Components|Box|GetScaledBoxExtent _spawnervolume))))
  (bind _returnvalue (Game|SpawnActorfromClass "/Game/Foraging/BP_Model.BP_Model_C" (Math|Transform|MakeTransform (Math|Vector|MakeVector (.x _output_get) (.y _output_get) 0.0) "0, 0, 0" "1.000000,1.000000,1.000000") "Undefined" "MultiplyWithRoot" 0 0))
  (bind _output_get_2 (Variables|/Game/Foraging/BP_Model.BP_Model_C|SetData _returnvalue (.OutItem (Utilities|Array|Random (Variables|Default|GetDataAssetArray)))))
  (Components|StaticMesh|SetStaticMesh (Variables|/Game/Foraging/BP_Model.BP_Model_C|GetStaticMesh _returnvalue) (Variables|/Game/Foraging/DataAsset/ForageItemDataAsset.ForageItemDataAsset_C|GetMesh _output_get_2)))

(event Input|ActionEvents|InputActionSpawnPickUp
  (params (Key :type Key%20Structure :default "None"))
  ;[0 0 0] Spawn Items
  (:Pressed
    (bind _returnvalue (Actor|GetActorOfClass "BP_Spawner_C"))
    (CallFunction|SpawnActor _returnvalue)))

(event Input|ActionEvents|InputActionDestroyPickUps
  (params (Key :type Key%20Structure :default "None"))
  ;[0 0 0] Destroy All Items (Testing)
  (:Pressed
    (bind _outactors (Actor|GetAllActorsOfClass "/Game/Foraging/BP_PickUpObject.BP_PickUpObject_C"))
    (for _array_element _outactors
      (Actor|DestroyActor _array_element))))

(fn ConstructionScript)

(fn RandomizePosition
  (bind _returnvalue (Transformation|GetActorTransform))
  (return (Math|Random|RandomFloatinRange (/ (.x (.location _returnvalue)) 2.0) (.x (.location _returnvalue))) (Math|Random|RandomFloatinRange (/ (.y (.location _returnvalue)) 2.0) (.y (.location _returnvalue))) (.z (.location _returnvalue)) (.rotation _returnvalue) (.scale _returnvalue)))