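; Forageable object that the player harvests with E while in range, replacing it with pickups.
; Overlap with BP_TopDownCharacter toggles the range flag, and its data asset sets the mesh at construction.
; Interaction spawns a random number of BP_PickUpObject actors at random offsets, passes each valid one the mesh and data asset, then destroys itself.
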(event Collision|EventActorBeginOverlap
  (params (OtherActor :type Actor%20Object%20Reference))
  ;[0 0 0] Check for overlap, sets bool  and adds the overlapped actor to the list
  (bind _asbp_top_down_character (Utilities|Casting|CastToBP_TopDownCharacter OtherActor))
  (if (Utilities|IsValid _asbp_top_down_character)
    (Variables|Default|SetisPlayerInRange true)))

(event Collision|EventActorEndOverlap
  (params (OtherActor :type Actor%20Object%20Reference))
  ;[0 0 0] Check if the player is exiting the collision
  (bind _asbp_top_down_character (Utilities|Casting|CastToBP_TopDownCharacter OtherActor))
  (if (Utilities|IsValid _asbp_top_down_character)
    (Variables|Default|SetisPlayerInRange false)))

(event Input|KeyboardEvents|E
  (params (Key :type Key%20Structure))
  ;[0 0 0] Checks for input from the player
  (:Pressed
    (if (Variables|Default|GetisPlayerInRange)
      (CallFunction|OnObjectInteract))))

(fn ConstructionScript
  (bind _data (Variables|Default|GetData)
    (:then
      (Components|StaticMesh|SetStaticMesh (Variables|Default|GetStaticMesh) (Variables|/Game/Foraging/DataAsset/ForageItemDataAsset.ForageItemDataAsset_C|GetMesh _data)))
    (:else)))

(fn OnObjectInteract
  ;[0 0 0] Destroy the object and instantiates X amount of pickups in random position
  (for _index (range 1 (Math|Random|RandomIntegerinRange 1 (Variables|Default|GetmaxSpawns)))
    (bind _returnvalue (Game|SpawnActorfromClass "/Game/Foraging/BP_PickUpObject.BP_PickUpObject_C" (Math|Conversions|ToTransform(Vector) (Math|Transform|TransformLocation (Math|Conversions|ToTransform(Vector) (Transformation|GetActorLocation)) (Math|Vector|MakeVector (Math|Random|RandomFloatinRange 5.0 2e+02) (Math|Random|RandomFloatinRange 5.0 1e+02) 0.0))) "Undefined" "MultiplyWithRoot" 0 0))
    ;[1 1 1] Valid check, that if player stands on the object, it won't immediately destroy it, causing problems.  Player will not pick up  the items either though.
    (Utilities|IsValid _returnvalue
      (:Is%20Valid
        ;[0 0 0] Passes Mesh, ID and Name to the spawned PickUpObjects
        (bind _data (Variables|Default|GetData)
          (:then
            (Components|StaticMesh|SetStaticMesh (Variables|/Game/Foraging/BP_PickUpObject.BP_PickUpObject_C|GetStaticMesh _returnvalue) (Variables|/Game/Foraging/DataAsset/ForageItemDataAsset.ForageItemDataAsset_C|GetMesh _data))
            (Variables|/Game/Foraging/BP_PickUpObject.BP_PickUpObject_C|SetSelectedDataAsset _returnvalue _data)
            (Actor|DestroyActor))
          (:else))))))