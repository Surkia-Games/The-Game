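; PlantHandler is an unfinished Blueprint for detecting a plant under the mouse cursor.
; A custom event, not called within this graph, traces WorldStatic objects under the cursor through the player controller and checks the hit actor for the "Plant" tag.
; A match and a left mouse press both lead to the same always-true branch, which does nothing.
; Disconnected visibility and debug print nodes remain, noted as not working.
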(event Custom|CustomEvent
  (params (DeltaSeconds :type Float%20%28single-precision%29))
  (bind _asplayer_controller (Utilities|Casting|CastToPlayerController (Pawn|GetController (Game|Player|GetPlayerPawn 0))))
  (if (.ReturnValue (Class|PlayerController|GetHitResultUnderCursorforObjects _asplayer_controller (Utilities|Array|MakeArray "ObjectTypeQuery1") true))
    (if (Actor|ActorHasTag (.HitActor (Collision|BreakHitResult (.HitResult (Class|PlayerController|GetHitResultUnderCursorforObjects _asplayer_controller (Utilities|Array|MakeArray "ObjectTypeQuery1") true)))) "Plant")
      (if true
        _))))

(event EventBeginPlay)

(event EventTick
  (params (DeltaSeconds :type Float%20%28single-precision%29)))

(event Input|MouseEvents|LeftMouseButton
  (params (Key :type Key%20Structure :default "None"))
  (:Pressed
    (if true
      _)))