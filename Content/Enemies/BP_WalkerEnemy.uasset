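; Walker enemy that roams the navmesh and heads toward where its AI Perception last sensed the player.
; TryMoveEnemy starts on BeginPlay, moving to the last stimulus location or, without one, a random nearby nav point.
; It re-issues the move every tick through AIMoveTo's immediate output and DelayUntilNextTick, without awaiting arrival.
; Perception updates store SeesPlayer and CurrentTargetPosition, which the movement logic never reads.
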(event EventBeginPlay
  ;[1 1 1] Calls itself.
  (CallFunction|TryMoveEnemy))

(event Collision|EventActorBeginOverlap
  (params (OtherActor :type Actor%20Object%20Reference)))

(event EventTick
  (params (DeltaSeconds :type Float%20%28single-precision%29)))

(event Custom|TryMoveEnemy
  (bind _self self)
  (bind _info (Class|AIPerceptionComponent|GetActorsPerception (Variables|Default|GetAIPerception) (Game|Player|GetPlayerPawn 0)))
  (if (> (Utilities|Array|LastIndex (.LastSensedStimuli (Utilities|Struct|BreakActorPerceptionBlueprintInfo _info))) -1)
    (AI|AIMoveTo _self (.RandomLocation (AI|Navigation|GetRandomReachablePointinRadius (.StimulusLocation (Utilities|Struct|BreakAIStimulus (Utilities|Array|Get(acopy) (.LastSensedStimuli (Utilities|Struct|BreakActorPerceptionBlueprintInfo _info)) (Utilities|Array|LastIndex (.LastSensedStimuli (Utilities|Struct|BreakActorPerceptionBlueprintInfo _info)))))) 0.0 0 0)) 0 5.0 false
      (:then
        (Utilities|FlowControl|DelayUntilNextTick)
        (CallFunction|TryMoveEnemy)))
    (else
      (bind _point (CallFunction|GetRandomNavPointAroundActor))
      (AI|AIMoveTo _self _point 0 5.0 false
        (:then
          (Utilities|FlowControl|DelayUntilNextTick)
          (CallFunction|TryMoveEnemy))))))

(event OnTargetPerceptionUpdated(AIPerception)
  (params (Actor :type Actor%20Object%20Reference) (Stimulus :type AI%20Stimulus%20Structure))
  (bind (_age _expirationage _strength _stimuluslocation _receiverlocation _tag _bsuccessfullysensed) (Utilities|Struct|BreakAIStimulus Stimulus))
  (Variables|Default|SetSeesPlayer _bsuccessfullysensed)
  (Variables|Default|SetCurrentTargetPosition _stimuluslocation))

(fn ConstructionScript)

(fn GetRandomNavPointAroundActor
  (bind _returnvalue (Transformation|GetActorLocation))
  (bind (_randomlocation _returnvalue_2) (AI|Navigation|GetRandomReachablePointinRadius _returnvalue 1e+03 0 0))
  (return _returnvalue_2 _randomlocation))